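; BP_GrapplePoint is a grapple hook anchor that tells the player character when it is within grapple range.
; Its Collider overlap events cast to BP_ThirdPersonCharacter and set or clear that character's IsPlayerInGrappleRange flag.
; While the player is inside, a point light becomes visible and a timeline pulses its intensity; leaving hides the light and stops the pulse.
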(event `self.Collider.OnComponentBeginOverlap`
  (params (OverlappedComponent :type "PrimitiveComponent Object Reference") (OtherActor :type "Actor Object Reference") (OtherComp :type "PrimitiveComponent Object Reference") (OtherBodyIndex :type Integer) (bFromSweep :type Boolean) (SweepResult :type "HitResult Structure (by ref)"))
  (bind _asbp_third_person_character (cast `/Game/ThirdPerson/Blueprints/BP_ThirdPersonCharacter` OtherActor))
  (set `/Game/ThirdPerson/Blueprints/BP_ThirdPersonCharacter.IsPlayerInGrappleRange` true _asbp_third_person_character)
  (`SceneComponent.SetVisibility` (`self.PointLight`) true false)
  (bind (_direction _pulseintensity) (`Timeline|PulseTimeline` :!label _label)
    (:`Update`
      (`LightComponent.SetIntensity` (`self.PointLight`) (* _pulseintensity 50000.0)))))

(event `self.Collider.OnComponentEndOverlap`
  (params (OverlappedComponent :type "PrimitiveComponent Object Reference") (OtherActor :type "Actor Object Reference") (OtherComp :type "PrimitiveComponent Object Reference") (OtherBodyIndex :type Integer))
  (bind _asbp_third_person_character (cast `/Game/ThirdPerson/Blueprints/BP_ThirdPersonCharacter` OtherActor))
  (set `/Game/ThirdPerson/Blueprints/BP_ThirdPersonCharacter.IsPlayerInGrappleRange` false _asbp_third_person_character)
  (`SceneComponent.SetVisibility` (`self.PointLight`) false false)
  (goto _label :!via `Stop`))

(fn `UserConstructionScript`)